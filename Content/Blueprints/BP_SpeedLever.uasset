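; BP_SpeedLever is a motion-controller-grabbable lever that slides along a spline, presumably as a speed control.
; GrabComponent's grab and drop events toggle IsGrabbed.
; While grabbed, Tick projects the controller position onto the spline, storing the distance along it in CurrentDist and moving the whole actor to the closest point.
; That point is requested in Local space but passed to SetActorLocation, which expects world space.
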(event OnGrabbed(GrabComponent)
  (Variables|Default|SetisGrabbed true))

(event OnDropped(GrabComponent)
  (Variables|Default|SetisGrabbed false))

(event EventBeginPlay)

(event EventTick
  (params (DeltaSeconds :type Float%20%28single-precision%29))
  (bind _grabcomponent (Variables|Default|GetGrabComponent))
  (bind _spline (Variables|Default|GetSpline))
  (bind _motioncontrollerref (Variables|/Game/VRTemplate/Blueprints/GrabComponent.GrabComponent_C|GetMotionControllerRef _grabcomponent))
  (bind _returnvalue (Transformation|GetWorldLocation _motioncontrollerref))
  (if (Variables|Default|GetisGrabbed)
    (Variables|Default|SetcurrentDist (Class|SplineComponent|GetDistanceAlongSplineatSplineInputKey _spline (Class|SplineComponent|FindInputKeyClosesttoWorldLocation _spline _returnvalue)))
    (Transformation|SetActorLocation (Spline|FindLocationClosesttoWorldLocation _spline _returnvalue "Local") false false)))

(fn ConstructionScript)
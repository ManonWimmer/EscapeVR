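; BP_Wheel is a wheel actor the player grabs and turns with a motion controller.
; GrabComponent events toggle the grabbed state, storing the controller and its starting angle on grab.
; While grabbed, Tick yaws SMWheel by the change in the controller's angle in wheel-local space (via atan2), scaled by delta time and Speed.
; It also draws a debug line along the wheel's up vector.
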(event OnGrabbed(GrabComponent)
  (params (MotionController :type Motion%20Controller%20Component%20Object%20Reference))
  ;[0 0.9952 1 0.5] Grabed
  (Utilities|IsValid MotionController
    (:Is%20Valid
      (if (not (Variables|Default|Getb_grabbed))
        (Variables|Default|Setb_grabbed true)
        (Variables|Default|SetMotion%20Controller MotionController)
        (bind _result (CallFunction|FComputeLookatWheelRotation))
        (Variables|Default|SetlastRot _result)))))

(event OnDropped(GrabComponent)
  ;[0 0.9952 1 0.5] Grabed
  (if (Variables|Default|Getb_grabbed)
    (Variables|Default|Setb_grabbed false)))

(event EventTick
  (params (DeltaSeconds :type Float%20%28single-precision%29))
  (bind _sm_wheel (Variables|Default|GetSM_Wheel))
  (bind _returnvalue (Transformation|GetWorldLocation _sm_wheel))
  ;[1 0.84 0.201 0.5] Tick
  (if (Variables|Default|Getb_grabbed)
    (Utilities|FlowControl|Sequence
      (:then_0
        (Rendering|Debug|DrawDebugLine _returnvalue (+ _returnvalue (* (Math|Vector|GetUpVector _sm_wheel) 2e+01)) "(R=1.000000,G=0.000000,B=0.162820,A=1.000000)" 5.0 0.0))
      (:then_1
        (bind _result (CallFunction|FComputeLookatWheelRotation))
        (Transformation|AddRelativeRotation (Variables|Default|GetSM_Wheel) (Math|Rotator|MakeRotator 0.0 0.0 (* (* (.yaw (Math|Rotator|MakeRotator (- (.roll _result) (.roll (Variables|Default|GetlastRot))) (- (.pitch _result) (.pitch (Variables|Default|GetlastRot))) (- (.yaw _result) (.yaw (Variables|Default|GetlastRot))))) (Utilities|Time|GetWorldDeltaSeconds)) (Variables|Default|Getspeed))) false false))
      (:then_2
        (bind _result_2 (CallFunction|FComputeLookatWheelRotation))
        (Variables|Default|SetlastRot _result_2)))))

(fn ConstructionScript)

(fn FComputeLookatWheelRotation
  (bind _sm_wheel (Variables|Default|GetSM_Wheel))
  (bind _motion_controller (Variables|Default|GetMotion%20Controller))
  (bind _returnvalue (Transformation|GetWorldTransform _sm_wheel))
  (bind _returnvalue_2 (Transformation|GetWorldLocation _motion_controller))
  (bind _returnvalue_3 (Math|Transform|InverseTransformLocation _returnvalue _returnvalue_2))
  (Utilities|IsValid _motion_controller
    (:Is%20Valid
      (return (Math|Rotator|MakeRotator 0.0 0.0 (Class|KismetMathLibrary|DegAtan2 (.y _returnvalue_3) (.x _returnvalue_3)))))))
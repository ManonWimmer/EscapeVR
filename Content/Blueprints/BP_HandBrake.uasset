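; BP_HandBrake is a VR handbrake lever that a motion controller grabs and rotates about its pivot, starting at BaseAngle.
; While held, Tick converts the controller position to pivot space and takes its XZ angle, clamped between BaseAngle and MaxAngle.
; Pitch eases toward that angle at a rate scaled by hand distance and frame time.
; On release it prints debug values and snaps to whichever end angle is nearer.
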(event OnGrabbed(GrabComponent)
  (params (MotionController :type Motion%20Controller%20Component%20Object%20Reference))
  (Variables|Default|SetMotion%20Controller MotionController))

(event OnDropped(GrabComponent)
  (bind _maxangle (Variables|Default|GetMaxAngle))
  (bind _baseangle (Variables|Default|GetBaseAngle))
  (bind _pivot (Variables|Default|GetPivot))
  (bind _pivot_2 (Variables|Default|GetPivot))
  (bind _relativerotation (Variables|/Script/Engine.SceneComponent|GetRelativeRotation _pivot_2))
  (bind _returnvalue (|((T-A)/(B-A)) (.pitch _relativerotation) _maxangle _baseangle))
  (Variables|Default|SetMotion%20Controller 0)
  (Development|PrintString (Utilities|String|Append (Utilities|String|ToString(Float) _returnvalue) "  Angle :" (Utilities|String|ToString(Float) (.pitch _relativerotation))))
  (if (< _returnvalue 0.5)
    (Transformation|SetRelativeRotation _pivot (Math|Rotator|MakeRotator 0.0 (Variables|Default|GetMaxAngle) 0.0) false false)
    (else
      (Transformation|SetRelativeRotation _pivot (Math|Rotator|MakeRotator 0.0 (Variables|Default|GetBaseAngle) 0.0) false false))))

(event EventTick
  (params (DeltaSeconds :type Float%20%28single-precision%29))
  (bind _motion_controller (Variables|Default|GetMotion%20Controller)
    (:then
      (Transformation|AddRelativeRotation (Variables|Default|GetPivot) (Math|Rotator|MakeRotator 0.0 (* (* (Math|Vector|VectorLengthXY (Math|Vector|MakeVector (.x (Math|Transform|InverseTransformLocation (Transformation|GetWorldTransform (Variables|Default|GetPivot)) (Transformation|GetWorldLocation _motion_controller))) (.z (Math|Transform|InverseTransformLocation (Transformation|GetWorldTransform (Variables|Default|GetPivot)) (Transformation|GetWorldLocation _motion_controller))) 0.0)) (- (Math|Float|Clamp(Float) (Class|KismetMathLibrary|DegAtan2 (.z (Math|Transform|InverseTransformLocation (Transformation|GetWorldTransform (Variables|Default|GetPivot)) (Transformation|GetWorldLocation _motion_controller))) (.x (Math|Transform|InverseTransformLocation (Transformation|GetWorldTransform (Variables|Default|GetPivot)) (Transformation|GetWorldLocation _motion_controller)))) (Variables|Default|GetBaseAngle) (Variables|Default|GetMaxAngle)) (.pitch (Variables|/Script/Engine.SceneComponent|GetRelativeRotation (Variables|Default|GetPivot))))) DeltaSeconds) 0.0) false false))
    (:else)))

(fn ConstructionScript
  (Transformation|SetRelativeRotation (Variables|Default|GetPivot) (Math|Rotator|MakeRotator 0.0 (Variables|Default|GetBaseAngle) 0.0) false false))
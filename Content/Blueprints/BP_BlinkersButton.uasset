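; Three-position blinker lever for VR, knocked up or down when a VRPawn component overlaps its box.
; The height difference between PivotPoint and the overlapping component picks the direction: contact from below pushes up, otherwise down.
; Each push steps a Position state between Up, Neutral and Down, snaps the pivot's pitch by RotationRange, and fires activate-up, activate-down or cancel on returning to Neutral.
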(event OnComponentBeginOverlap(Box)
  (params (OverlappedComponent :type Primitive%20Component%20Object%20Reference) (OtherActor :type Actor%20Object%20Reference) (OtherComp :type Primitive%20Component%20Object%20Reference) (OtherBodyIndex :type Integer) (bFromSweep :type Boolean) (SweepResult :type Hit%20Result%20Structure%20%28by%20ref%29))
  (bind _returnvalue (Transformation|GetWorldLocation OtherComp))
  (bind _pivotpoint (Variables|Default|GetPivotPoint))
  (bind _returnvalue_2 (Transformation|GetWorldLocation _pivotpoint))
  (bind _returnvalue_3 (- _returnvalue_2 _returnvalue))
  (bind _returnvalue_4 (Math|Vector|DotProduct _returnvalue_3 "0.000000,0.000000,1.000000"))
  ;[0.05163 0.04912 0.15 0.5] Collisions
  (Utilities|Casting|CastToVRPawn OtherActor)
  (Development|PrintString "Collided")
  (if (> _returnvalue_4 0.1)
    (CallFunction|CEActivateUp)
    (elif (< _returnvalue_4 0.1)
      (CallFunction|CEActivateDown))))

(event Custom|CE_Activate_Up
  ;[0.15 0.04986 0.04628 0.5] Custom Events
  (switch Utilities|FlowControl|Switch|SwitchonE_Blinkers (Variables|Default|GetPosition)
    (:NewEnumerator1
      (Variables|Default|SetPosition "NewEnumerator0")
      (Transformation|SetRelativeRotation (Variables|Default|GetPivotPoint) (Math|Rotator|MakeRotator 0.0 (- 0.0 (Variables|Default|GetRotationRange)) 0.0) false false)
      (Default|CallOnActivateUp))
    (:NewEnumerator2
      (Variables|Default|SetPosition "NewEnumerator1")
      (Transformation|SetRelativeRotation (Variables|Default|GetPivotPoint) "0.0,0.0,0.0" false false)
      (Default|CallOnCancel))))

(event Custom|CE_Activate_Down
  ;[0.15 0.04986 0.04628 0.5] Custom Events
  (switch Utilities|FlowControl|Switch|SwitchonE_Blinkers (Variables|Default|GetPosition)
    (:NewEnumerator0
      (Variables|Default|SetPosition "NewEnumerator1")
      (Transformation|SetRelativeRotation (Variables|Default|GetPivotPoint) "0, 0, 0" false false)
      (Default|CallOnCancel))
    (:NewEnumerator1
      (Variables|Default|SetPosition "NewEnumerator2")
      (Transformation|SetRelativeRotation (Variables|Default|GetPivotPoint) (Math|Rotator|MakeRotator 0.0 (Variables|Default|GetRotationRange) 0.0) false false)
      (Default|CallOnActivateDown))))

(fn ConstructionScript)
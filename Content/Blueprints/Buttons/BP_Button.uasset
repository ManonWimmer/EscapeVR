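; BP_Button is a pressure button that toggles its pressed state as overlaps begin and end on its trigger.
; Each state change calls the OnPressed dispatcher and plays or reverses a timeline that lerps the button mesh between rest and offset positions.
; The timeline's rate derives from ButtonPressedEffect, and every update also plays a bip sound.
; CE_Press and CE_Unpress drive only the visual, without changing state or broadcasting.
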(event OnComponentBeginOverlap(Trigger)
  (params (OverlappedComponent :type Primitive%20Component%20Object%20Reference) (OtherActor :type Actor%20Object%20Reference) (OtherComp :type Primitive%20Component%20Object%20Reference) (OtherBodyIndex :type Integer) (bFromSweep :type Boolean) (SweepResult :type Hit%20Result%20Structure%20%28by%20ref%29))
  ;[0.1327 0.9795 1 0.5] Overlaps
  (if (not (Variables|Default|Getb_pressed))
    (bind _output_get (Variables|Default|Setb_pressed true))
    (Default|CallOnPressed _output_get)
    (CallFunction|CEUpdatePressedVIsual _output_get)))

(event OnComponentEndOverlap(Trigger)
  (params (OverlappedComponent :type Primitive%20Component%20Object%20Reference) (OtherActor :type Actor%20Object%20Reference) (OtherComp :type Primitive%20Component%20Object%20Reference) (OtherBodyIndex :type Integer))
  ;[0.1327 0.9795 1 0.5] Overlaps
  (if (Variables|Default|Getb_pressed)
    (bind _output_get (Variables|Default|Setb_pressed false))
    (Default|CallOnPressed _output_get)
    (CallFunction|CEUpdatePressedVIsual _output_get)))

(event Custom|CE_UpdatePressedVIsual
  (params (Pressed :type Boolean))
  ;[0.9781 0.2529 0.922 0.5] Update Pressed Visuals
  (if Pressed
    (bind _zpos_lerp (Timeline|TL_ButtonEffect Play)
      (:Update
        (Transformation|SetRelativeLocation (Variables|Default|GetBtn) (Math|Vector|Lerp(Vector) (Variables|Default|GetstartPos) (+ (Variables|Default|GetstartPos) (Variables|Default|GetpressedPos)) _zpos_lerp) false false)
        (Audio|PlaySoundatLocation "/Game/Assets/Sounds/Button/MS_SFX_Bip.MS_SFX_Bip" (Transformation|GetActorLocation) "0, 0, 0" 1.0 1.0 0.0 0 0 0 0)))
    (else
      (Timeline|TL_ButtonEffect Reverse))))

(event Custom|CE_Unpress
  (CallFunction|CEUpdatePressedVIsual false))

(event Custom|CE_Press
  (CallFunction|CEUpdatePressedVIsual true))

(event EventBeginPlay
  ;[0.225 1 0.3294 0.5] Begin
  (Variables|Default|SetstartPos (Variables|/Script/Engine.SceneComponent|GetRelativeLocation (Variables|Default|GetBtn)))
  (Components|Timeline|SetPlayRate (Variables|Default|GetTL_ButtonEffect) (/ 1.0 (Variables|Default|GetButtonPressedEffect))))

(fn ConstructionScript)
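; BP_Wiper is a wiper whose speed is set by a three-position side lever: fast, normal or off.
; A self-restarting timeline drives the pitch of the Pivot through CalcAngle, with the play rate taken from the lever's speed.
; Speed is read only between cycles, so a running sweep finishes before a change applies, and the off state polls on a short delay.
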(event Custom|CE_OnPositionChange
  (params (NewParam :type E_Blinkers%20Enum :default "NewEnumerator0"))
  (switch Utilities|FlowControl|Switch|SwitchonE_Blinkers NewParam
    (:NewEnumerator0
      (Variables|Default|SetCurrentSpeed 2))
    (:NewEnumerator1
      (Variables|Default|SetCurrentSpeed 1))
    (:NewEnumerator2
      (Variables|Default|SetCurrentSpeed 0))))

(event Custom|CE_StartTimeline
  (if (!= (Variables|Default|GetCurrentSpeed) 0)
    (Components|Timeline|SetPlayRate (Variables|Default|GetTimeline) (Math|Conversions|ToFloat(Integer) (Variables|Default|GetCurrentSpeed)))
    (bind _value (Timeline|Timeline PlayFromStart)
      (:Update
        (Transformation|SetRelativeRotation (Variables|Default|GetPivot) (Math|Rotator|MakeRotator 0.0 (Utilities|CalcAngle _value) 0.0) false false))
      (:Finished
        (CallFunction|CEStartTimeline)))
    (else
      (Utilities|FlowControl|Delay 0.1)
      (CallFunction|CEStartTimeline))))

(event EventBeginPlay
  (EventDispatchers|BindEventtoOnPositionChange (Variables|Default|GetSideLever) (delegate Custom|CE_OnPositionChange))
  (CallFunction|CEStartTimeline))

(fn ConstructionScript)
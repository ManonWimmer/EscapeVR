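; TchouTchou is a VR grabbable pull handle that slides vertically between the two ends of a spline.
; While grabbed, a looping timer moves the capsule to follow the motion controller's Z, clamped to the spline points, and prints the value.
; When released, Tick eases it back to the first point's height.
; BeginPlay starts a fire sound at zero volume, but its volume-update event is empty.
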(event OnGrabbed(GrabComponent)
  (params (MotionController :type Motion%20Controller%20Component%20Object%20Reference))
  ;[0.069 0.15 0.1351 0.5] Grabbed - Move Z
  (Variables|Default|SetMotion%20Controller MotionController)
  (bind _returnvalue (Utilities|Time|SetTimerbyFunctionName 0 "UpdatePosition" 0.01 true true))
  (Variables|Default|SetTimer _returnvalue)
  (Variables|Default|SetIsGrabbed true))

(event OnDropped(GrabComponent)
  ;[0.069 0.15 0.1351 0.5] Grabbed - Move Z
  (Utilities|Time|ClearandInvalidateTimerbyHandle (Variables|Default|GetTimer))
  (Variables|Default|SetMotion%20Controller 0)
  (Variables|Default|SetIsGrabbed false))

(event Custom|CE_UpdateSoundVolume)

(event EventTick
  (params (DeltaSeconds :type Float%20%28single-precision%29))
  (bind _capsule (Variables|Default|GetCapsule))
  (bind _relativelocation (Variables|/Script/Engine.SceneComponent|GetRelativeLocation _capsule))
  ;[0.15 0.01596 0.08022 0.5] Not Grabbed - Move back to pos Z
  (if (not (Variables|Default|GetIsGrabbed))
    (Transformation|SetRelativeLocation _capsule (Math|Interpolation|VInterpTo (Variables|/Script/Engine.SceneComponent|GetRelativeLocation _capsule) (Math|Vector|MakeVector (.x _relativelocation) (.y _relativelocation) (.z (Spline|GetLocationatSplinePoint (Variables|Default|GetSpline) 0 "Local"))) DeltaSeconds (Variables|Default|GetBackToPosSpeed)) false false)
    (CallFunction|CEUpdateSoundVolume)))

(event EventBeginPlay
  ;[0.15 0.1417 0.04362 0.5] Setup Sound
  (bind _returnvalue (Audio|SpawnSoundatLocation "/Game/VRTemplate/Audio/Fire01.Fire01" (Transformation|GetWorldLocation (Variables|Default|GetScene)) "0, 0, 0" 0.0 1.0 0.0 0 0))
  (bind _output_get (Variables|Default|SetTchouTchouSound _returnvalue))
  (Audio|Components|Audio|Play _output_get 0.0))

(fn ConstructionScript)

(fn UpdatePosition
  (bind _motion_controller (Variables|Default|GetMotion%20Controller))
  (bind _spline (Variables|Default|GetSpline))
  (bind _capsule (Variables|Default|GetCapsule))
  (bind _returnvalue (Transformation|GetWorldTransform _motion_controller))
  (bind _returnvalue_2 (Spline|GetLocationatSplinePoint _spline 1 "Local"))
  (bind _returnvalue_3 (Spline|GetLocationatSplinePoint _spline 0 "Local"))
  (bind _returnvalue_4 (Transformation|GetWorldTransform _capsule))
  (bind _relativelocation (Variables|/Script/Engine.SceneComponent|GetRelativeLocation _capsule))
  (bind _returnvalue_5 (Math|Transform|MakeRelativeTransform _returnvalue _returnvalue_4))
  (bind _returnvalue_6 (+ (.z _relativelocation) (.z (.location _returnvalue_5))))
  (bind _returnvalue_7 (Math|Float|Clamp(Float) _returnvalue_6 (.z _returnvalue_2) (.z _returnvalue_3)))
  (Transformation|SetRelativeLocation _capsule (Math|Vector|MakeVector (.x _relativelocation) (.y _relativelocation) _returnvalue_7) false false)
  (Development|PrintText (Utilities|Text|ToText(Float) _returnvalue_7 "HalfToEven")))
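; BP_Blinker is a left or right blinker indicator that shows its active state on a sphere mesh in response to a BlinkerButton.
; On BeginPlay it creates a dynamic material instance for the sphere and binds to the button's cancel event.
; IsRight selects whether it also listens for the button's activate-up or activate-down event.
; The bound events switch the material's IsActive scalar parameter on or off.
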(event Custom|CE_Activate
  (Rendering|Material|SetScalarParameterValue (Variables|Default|GetMaterial) "IsActive" 1.0 :!class /Script/Engine.MaterialInstanceDynamic))

(event Custom|CE_Cancel
  (Rendering|Material|SetScalarParameterValue (Variables|Default|GetMaterial) "IsActive" 0.0 :!class /Script/Engine.MaterialInstanceDynamic))

(event EventBeginPlay
  (bind _sphere (Variables|Default|GetSphere))
  (bind _returnvalue (Rendering|Material|CreateDynamicMaterialInstance _sphere 0 (Rendering|Material|GetMaterial _sphere 0) "None" :!class /Script/Engine.PrimitiveComponent))
  (Variables|Default|SetMaterial _returnvalue)
  (EventDispatchers|BindEventtoOnCancel (Variables|Default|GetBlinkerButton) (EventDispatchers|CreateEvent :!event Custom|CE_Cancel))
  (if (Variables|Default|GetIsRight)
    (EventDispatchers|BindEventtoOnActivateUp (Variables|Default|GetBlinkerButton) (EventDispatchers|CreateEvent :!event Custom|CE_Activate))
    (else
      (EventDispatchers|AssignOnActivateDown (Variables|Default|GetBlinkerButton) (EventDispatchers|CreateEvent :!event Custom|CE_Activate)))))

(fn ConstructionScript)
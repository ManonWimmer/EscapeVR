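; Grabbable seatbelt Blueprint for motion controllers that the player pulls to a buckle to fasten.
; When the latch plate overlaps the buckle collider while held, a dispatcher fires, releasing the grab, snapping the capsule onto the buckle and playing a sound.
; Until buckled, Tick eases a released belt back to its BeginPlay position and toward zero rotation.
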(event OnComponentBeginOverlap(BuckleCollider)
  (params (OverlappedComponent :type Primitive%20Component%20Object%20Reference) (OtherActor :type Actor%20Object%20Reference) (OtherComp :type Primitive%20Component%20Object%20Reference) (OtherBodyIndex :type Integer) (bFromSweep :type Boolean) (SweepResult :type Hit%20Result%20Structure%20%28by%20ref%29))
  ;[0.15 0.1211 0.02908 0.5] Buckle overlapped by latch plate
  (Utilities|IsValid (Variables|Default|GetMotion%20Controller)
    (:Is%20Valid
      (if (== OtherComp (Variables|Default|GetLatchPlate))
        (Default|CallOnSeatbeltBuckled)))))

(event OnGrabbed(GrabComponent)
  (params (MotionController :type Motion%20Controller%20Component%20Object%20Reference))
  ;[0.15 0.04825 0.09437 0.5] Grab / Drop
  (Variables|Default|SetMotion%20Controller MotionController)
  (Variables|Default|SetIsGrabbed true))

(event OnDropped(GrabComponent)
  ;[0.15 0.04825 0.09437 0.5] Grab / Drop
  (Variables|Default|SetMotion%20Controller 0)
  (Variables|Default|SetIsGrabbed false))

(event Custom|CE_Buckle
  ;[0.15 0.04637 0.04534 0.5] Buckle : set pos in buckle + sound
  (Default|TryRelease (Variables|Default|GetGrabComponent))
  (Transformation|AttachComponentToComponent (Variables|Default|GetCapsule) (Variables|Default|GetBuckle) "None" "KeepRelative" "KeepRelative" "KeepRelative" true)
  (Transformation|SetRelativeLocation (Variables|Default|GetCapsule) "0, 0, 0" false false)
  (Variables|Default|SetHasBeenBuckled true)
  (Audio|PlaySoundatLocation "/Game/Assets/Sounds/seatbelt_buckled.seatbelt_buckled" (Transformation|GetWorldLocation (Variables|Default|GetBuckle)) "0, 0, 0" 1.0 1.0 0.0 0 0 0 0))

(event EventBeginPlay
  (Variables|Default|SetStartPos (Transformation|GetWorldLocation (Variables|Default|GetCapsule)))
  ;[0.15 0.04637 0.04534 0.5] Buckle : set pos in buckle + sound
  (EventDispatchers|BindEventtoOnSeatbeltBuckled (delegate Custom|CE_Buckle)))

(event EventTick
  (params (DeltaSeconds :type Float%20%28single-precision%29))
  (bind _capsule (Variables|Default|GetCapsule))
  (bind _backtoposspeed (Variables|Default|GetBackToPosSpeed))
  ;[0.07096 0.04909 0.15 0.5] Seatbelt back to pos on dropped not on buckle
  (if (and (not (Variables|Default|GetIsGrabbed)) (not (Variables|Default|GetHasBeenBuckled)))
    (Transformation|SetWorldLocationAndRotation _capsule (Math|Interpolation|VInterpTo (Transformation|GetWorldLocation _capsule) (Variables|Default|GetStartPos) DeltaSeconds _backtoposspeed) (Math|Interpolation|RInterpTo (Transformation|GetWorldRotation _capsule) "0, 0, 0" DeltaSeconds _backtoposspeed) false false)))

(fn ConstructionScript)